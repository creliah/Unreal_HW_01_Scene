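; Game mode Blueprint (遊戲模式) that runs a minutes-and-seconds countdown and pauses the game when time runs out.
; Event Tick feeds a one-second Delay, which ignores re-triggers while pending, so seconds (秒) drop about once per second.
; When seconds fall below zero they wrap to 59 and minutes (分) decrement.
; With no minutes left, seconds reset to zero and the game pauses.
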(event EventTick
  (params (DeltaSeconds :type Float%20%28single-precision%29))
  ;[1 0.5221 0.4039] 倒數系統
  ;;[1 1 1] 每秒秒數減一
  (Utilities|FlowControl|Delay 1.0) ; 延遲：等待所設定的時間再執行後面的節點
  (bind _output_get (Variables|Default|Set秒 (- (Variables|Default|Get秒) 1)))
  ;;[1 1 1] 當秒數低於0，就將秒數設為59
  (if (< _output_get 0) ; 判斷：\n當布林值\n為正確則從True出去\n為錯誤則從False
    (Variables|Default|Set秒 59)
    ;;[1 1 1] 分大於0時，分-1
    (if (> (Variables|Default|Get分) 0)
      (Variables|Default|Set分 (- (Variables|Default|Get分) 1))
      (else
        ;;[1 1 1] 當分=0時，秒=59。時間停止時，秒數為0並將遊戲暫停。
        (if (== (Variables|Default|Get秒) 59)
          (Variables|Default|Set秒 0)
          (Game|SetGamePaused true))))))

(fn ConstructionScript)